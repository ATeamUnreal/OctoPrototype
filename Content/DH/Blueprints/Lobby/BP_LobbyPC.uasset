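; BP_LobbyPC is the lobby player controller that creates the lobby widget and moves the session into the game level.
; On BeginPlay it adds the widget, shows the cursor and sets Game and UI input.
; The authority writes the PlayerArray count to BP_LobbyGS.UserCount, while remote clients hide the start button.
; GameStart waits briefly, then runs a servertravel console command so the host brings all players to Level1.
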(event Custom|SetupWidget
  (bind _returnvalue (UserInterface|CreateWidget "/Game/DH/Blueprints/Lobby/LobbyWidget.LobbyWidget_C"))
  (Variables|Default|SetLobbyWidget _returnvalue)
  (UserInterface|Viewport|AddtoViewport _returnvalue 0)
  (Networking|SwitchHasAuthority
    (:Authority
      (bind _asbp_lobby_gs (Utilities|Casting|CastToBP_LobbyGS (Game|GetGameState)))
      (Utilities|IsValid _asbp_lobby_gs
        (:Is%20Valid
          (Variables|/Game/DH/Blueprints/Lobby/BP_LobbyGS.BP_LobbyGS_C|SetUserCount _asbp_lobby_gs (Utilities|Array|Length (Variables|/Script/Engine.GameStateBase|GetPlayerArray _asbp_lobby_gs))))))
    (:Remote
      (Default|HideStartButton _returnvalue))))

(event Custom|GameStart
  ;[1 1 1] 서버 호스트가 다른 플레이어들 데리고 맵이동을 하는 개념이라고 합니다
  (Utilities|FlowControl|Delay 0.2)
  (Development|ExecuteConsoleCommand "servertravel/Game/Maps/Level1" 0))

(event EventBeginPlay
  (CallFunction|SetupWidget)
  (Variables|Default|SetbShowMouseCursor true)
  (Input|SetInputModeGameandUI self 0 "DoNotLock" true))

(event EventTick
  (params (DeltaSeconds :type Float%20%28single-precision%29)))

(fn ConstructionScript)