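; Player controller that picks a pawn class and character widget based on whether the local player is the server or a client.
; On BeginPlay it sets game-only input, then uses an authority switch to show the matching widget and call ServerSetPawn.
; That event stores the class, exposed through GetPlayerPawnClass, and has BP_MainGM restart the player.
; Both pawn slots currently hold BP_PlayerCharacter, assigned in the construction script.
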(event Custom|DeterminePawnClass
  (if (Pawn|IsLocalController)
    ;[1 1 1] 서버인지 클라인지 구분하려 pawn과 UI 표시
    (Networking|SwitchHasAuthority
      (:Authority
        (CallFunction|ServerSetPawn (Variables|Default|GetPawnToUseA))
        (bind _returnvalue (UserInterface|CreateWidget "/Game/DH/Blueprints/Main/ServerCharacterWidget.ServerCharacterWidget_C"))
        (UserInterface|Viewport|AddtoViewport _returnvalue 0))
      (:Remote
        (CallFunction|ServerSetPawn (Variables|Default|GetPawnToUseB))
        (bind _returnvalue_2 (UserInterface|CreateWidget "/Game/DH/Blueprints/Main/ClientCharacterWidget.ClientCharacterWidget_C"))
        (UserInterface|Viewport|AddtoViewport _returnvalue_2 0)))))

(event Custom|ServerSetPawn
  (params (InPawnClass :type Pawn%20Class%20Reference))
  (Variables|Default|SetMyPawnClass InPawnClass)
  (bind _asbp_main_gm (Utilities|Casting|CastToBP_MainGM (Game|GetGameMode)))
  (Class|GameModeBase|RestartPlayer _asbp_main_gm self))

(event EventBeginPlay
  (Variables|Default|SetbShowMouseCursor false)
  (Input|SetInputModeGameOnly self)
  (CallFunction|DeterminePawnClass)
  (if (Pawn|IsLocalController)
    (Development|PrintString (Utilities|GetDisplayName self))))

(fn ConstructionScript
  ;[1 1 1] 사용할 폰을 미리 등록
  (Variables|Default|SetPawnToUseA "/Game/DH/Blueprints/BP_PlayerCharacter.BP_PlayerCharacter_C")
  (Variables|Default|SetPawnToUseB "/Game/DH/Blueprints/BP_PlayerCharacter.BP_PlayerCharacter_C")
  (Networking|SetReplicates true))

(fn GetPlayerPawnClass
  (return (Variables|Default|GetMyPawnClass)))