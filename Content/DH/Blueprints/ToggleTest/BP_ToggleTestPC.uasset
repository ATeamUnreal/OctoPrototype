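; Test player controller that toggles the player between VR and non-VR play at runtime.
; E enables HMD and stereo through console commands and swaps to BP_VRPawn; Q disables them and swaps to BP_MyCharacter.
; Each swap unpossesses and destroys the current pawn, then spawns and possesses the new one at its saved location and rotation with unit scale, enabling movement replication.
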(event Custom|EnableVR
  (Development|ExecuteConsoleCommand "vr.bEnableHMD True" 0)
  (Development|ExecuteConsoleCommand "vr.bEnableStereo True" 0))

(event Custom|DisableVR
  (Development|ExecuteConsoleCommand "vr.bEnableStereo False" 0)
  (Development|ExecuteConsoleCommand "vr.bEnableHMD False" 0))

(event EventBeginPlay)

(event EventTick
  (params (DeltaSeconds :type Float%20%28single-precision%29)))

(event Input|KeyboardEvents|E
  (params (Key :type Key%20Structure))
  (bind _self self)
  (:Pressed
    (Development|PrintString "E")
    (CallFunction|EnableVR)
    (bind _spawn_transform (CallFunction|DestroyandUnpossessControllersPawn _self))
    (CallFunction|SpawnandPossessPawn "/Game/DH/Blueprints/VRMultiTest/BP_VRPawn.BP_VRPawn_C" _spawn_transform _self)))

(event Input|KeyboardEvents|Q
  (params (Key :type Key%20Structure))
  (bind _self self)
  (:Pressed
    (Development|PrintString "Q")
    (CallFunction|DisableVR)
    (bind _spawn_transform (CallFunction|DestroyandUnpossessControllersPawn _self))
    (CallFunction|SpawnandPossessPawn "/Game/DH/Blueprints/Main/BP_MyCharacter.BP_MyCharacter_C" _spawn_transform _self)))

(fn ConstructionScript)

(fn DestroyandUnpossessControllersPawn
  (params (PlayerController :type Player%20Controller%20Object%20Reference))
  (bind _output_get (LocalVariables|SetCurrentPlayerController PlayerController))
  (Utilities|IsValid (Pawn|GetControlledPawn _output_get)
    (:Is%20Valid
      (LocalVariables|SetCurrentPawn (Pawn|GetControlledPawn _output_get))
      (bind _output_get_2 (LocalVariables|SetPawn%20Transform (Math|Transform|MakeTransform (.location (Transformation|GetActorTransform (Pawn|GetControlledPawn _output_get))) (.rotation (Transformation|GetActorTransform (Pawn|GetControlledPawn _output_get))) "1,1,1")))
      (Pawn|UnPossess (LocalVariables|GetCurrentPlayerController))
      (Actor|DestroyActor (LocalVariables|GetCurrentPawn)))
    (:Is%20Not%20Valid
      (Pawn|UnPossess (LocalVariables|GetCurrentPlayerController))))
  (return _output_get_2))

(fn SpawnandPossessPawn
  (params (PawnClass :type Pawn%20Class%20Reference) (SpawnTransform :type Transform) (PlayerController :type Player%20Controller%20Object%20Reference))
  (bind _returnvalue (Game|SpawnActorfromClass PawnClass SpawnTransform "Undefined" PlayerController 0))
  (bind _aspawn (Utilities|Casting|CastToPawn _returnvalue))
  (Pawn|Possess PlayerController _aspawn)
  (Class|Actor|SetReplicateMovement _aspawn true))