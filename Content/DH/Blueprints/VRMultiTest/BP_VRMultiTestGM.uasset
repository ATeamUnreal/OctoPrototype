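; BP_VRMultiTestGM is a game mode for a VR multiplayer test that gives each joining player its own pawn.
; On PostLogin it picks a pawn class and spawn transform by a running player index, BP_Pawn1 for the first and BP_MyCharacter for the second.
; It spawns and possesses that pawn, enables movement replication, advances the index and prints the pawn's name.
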(event EventPostLogin
  (params (NewPlayer :type Player%20Controller%20Object%20Reference))
  (bind _playerindex (Variables|Default|GetPlayerIndex))
  (bind _returnvalue (Game|SpawnActorfromClass (Utilities|Select :Index _playerindex :Option%200 "/Game/IKTest/BP_Pawn1.BP_Pawn1_C" :Option%201 "/Game/DH/Blueprints/Main/BP_MyCharacter.BP_MyCharacter_C") (Utilities|Select :Index _playerindex :Option%200 (Math|Transform|MakeTransform "0, 0,80.000000") :Option%201 (Math|Transform|MakeTransform "-340.000000,30.000000,127.000000")) "AlwaysSpawn" 0 0))
  (bind _aspawn (Utilities|Casting|CastToPawn _returnvalue))
  (Pawn|Possess NewPlayer _aspawn)
  (Class|Actor|SetReplicateMovement _aspawn true)
  (Math|Integer|IncrementInt (Variables|Default|GetPlayerIndex)
    (:%20%20
      (Development|PrintString (Utilities|GetDisplayName _aspawn) true true "(R=0.249593,G=1.000000,B=0.000000,A=1.000000)" 1e+01))))

(fn ConstructionScript)

(fn DestroyandUnpossessControllersPawn)