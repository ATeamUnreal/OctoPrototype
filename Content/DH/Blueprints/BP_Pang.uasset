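; BP_Pang is a spinning weapon pickup that arms the player when overlapped.
; Each tick it adds a local rotation scaled by WeaponRotateSpeed and delta time.
; On any actor overlap, it casts player 0's character to BP_PlayerCharacter without checking the overlapping actor, calls WeaponAttachment on it, then destroys itself.
; A node that disables Box collision is present but never runs.
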(event EventTick
  (params (DeltaSeconds :type Float%20%28single-precision%29))
  ;[1 1 1] WeaponRotation
  (Transformation|AddActorLocalRotation (* (Variables|Default|GetWeaponRotateSpeed) (Utilities|Time|GetWorldDeltaSeconds)) false false))

(event Collision|EventActorBeginOverlap
  (params (OtherActor :type Actor%20Object%20Reference))
  (bind _asbp_player_character (Utilities|Casting|CastToBP_PlayerCharacter (Game|GetPlayerCharacter 0)))
  (Default|WeaponAttachment _asbp_player_character)
  (Actor|DestroyActor))

(fn ConstructionScript)