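; BP_GameGM is a game mode that gives each joining player a pawn chosen by join order.
; On PostLogin, a PlayerIndex counter selects class and spawn transform: BP_Pawn1 for index zero, BP_MyCharacterPUBGSimple for the other four options, with later slots offset along Y.
; The spawn ignores collisions, then the new player possesses the pawn and the counter increments.
; An unconnected branch that would shrink pawns after the first never runs.
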(event EventPostLogin
  (params (NewPlayer :type Player%20Controller%20Object%20Reference))
  (bind _playerindex (Variables|Default|GetPlayerIndex))
  (bind _returnvalue (* _playerindex 5e+01))
  (bind _returnvalue_2 (Math|Vector|MakeVector 4.5e+02 _returnvalue 0.0))
  (bind _returnvalue_3 (Math|Transform|MakeTransform _returnvalue_2 "0,180.000000, 0"))
  (bind _returnvalue_4 (Game|SpawnActorfromClass (Utilities|Select :Index (Variables|Default|GetPlayerIndex) :Option%200 "/Game/SH/SH_Stretch/BP/BP_Pawn1.BP_Pawn1_C" :Option%201 "/Game/SH/SH_Stretch/BP/BP_MyCharacterPUBGSimple.BP_MyCharacterPUBGSimple_C" :Option%202 "/Game/SH/SH_Stretch/BP/BP_MyCharacterPUBGSimple.BP_MyCharacterPUBGSimple_C" :Option%203 "/Game/SH/SH_Stretch/BP/BP_MyCharacterPUBGSimple.BP_MyCharacterPUBGSimple_C" :Option%204 "/Game/SH/SH_Stretch/BP/BP_MyCharacterPUBGSimple.BP_MyCharacterPUBGSimple_C") (Utilities|Select :Index (Variables|Default|GetPlayerIndex) :Option%200 (Math|Transform|MakeTransform "0, 0,400.000000") :Option%201 (Math|Transform|MakeTransform "23.000000,-277.000000,394.000000") :Option%202 _returnvalue_3 :Option%203 _returnvalue_3 :Option%204 _returnvalue_3) "AlwaysSpawn" 0 0))
  (bind _aspawn (Utilities|Casting|CastToPawn _returnvalue_4))
  (Utilities|IsValid _aspawn
    (:Is%20Valid
      (Pawn|Possess NewPlayer _aspawn)
      (Math|Integer|IncrementInt (Variables|Default|GetPlayerIndex)))))

(fn ConstructionScript)