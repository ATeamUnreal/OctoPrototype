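; VR player pawn that sets the tracking origin per headset and spawns left and right BP_MotionController actors attached to the VR origin.
; Grab and stretch inputs for each hand call that controller's grab, release or FireHand.
; Tick derives climbing and falling flags from the ClimbingHands count.
; The climbing gravity trace and hand transform update are disconnected, so falling never moves the pawn here.
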(event EventTick
  (params (DeltaSeconds :type Float%20%28single-precision%29))
  ;[1 1 1] 클라이밍
  (if (<= (Variables|Default|GetClimbingHands) 0)
    (if (Variables|Default|GetIsFalling)
      (Variables|Default|SetClimbingHands 0)
      (elif (Variables|Default|GetIsClimbing)
        (Variables|Default|SetIsClimbing false)
        (Variables|Default|SetIsFalling true)
        (else
          (Variables|Default|SetClimbingHands 0))))
    (else
      (Variables|Default|SetIsClimbing true)
      (Variables|Default|SetIsFalling false))))

(event EventBeginPlay
  (bind _returnvalue (Math|Transform|MakeTransform "0, 0, 0"))
  (bind _self self)
  (Utilities|FlowControl|Sequence
    (:then_0
      ;[1 1 1] Setup Player Height for various Platforms
      (switch name (Class|HeadMountedDisplayFunctionLibrary|GetHMDDeviceName)
        (:OculusHMD
          (Class|HeadMountedDisplayFunctionLibrary|SetTrackingOrigin "Floor" :!label _label))
        (:SteamVR
          (goto _label))
        (:PSVR
          (Class|HeadMountedDisplayFunctionLibrary|SetTrackingOrigin "Eye")
          (Transformation|AddLocalOffset (Variables|Default|GetVROrigin) (Math|Vector|MakeVector 0.0 0.0 (Variables|Default|GetDefaultPlayerHeight)) false false))))
    (:then_1
      ;[1 1 1] Spwan and attach both motion controllers
      (Utilities|FlowControl|Sequence
        (:then_0
          (bind _returnvalue_2 (Game|SpawnActorfromClass "/Game/SH/SH_Stretch/BP/BP_MotionController.BP_MotionController_C" _returnvalue "Undefined" _self "Left" 0))
          (Variables|Default|SetLeftController _returnvalue_2)
          (Transformation|AttachComponentToComponent _returnvalue_2 (Variables|Default|GetVROrigin) "None" "SnapToTarget" "SnapToTarget" "KeepWorld" false))
        (:then_1
          (bind _returnvalue_3 (Game|SpawnActorfromClass "/Game/SH/SH_Stretch/BP/BP_MotionController.BP_MotionController_C" _returnvalue "Undefined" _self "Right" 0))
          (Variables|Default|SetRightController _returnvalue_3)
          (Transformation|AttachComponentToComponent _returnvalue_3 (Variables|Default|GetVROrigin) "None" "SnapToTarget" "SnapToTarget" "KeepWorld" false))))))

(event Input|ActionEvents|InputActionGrabLeft
  (params (Key :type Key%20Structure))
  (bind _leftcontroller (Variables|Default|GetLeftController))
  ;[1 1 1] 좌측 컨트롤러 입력
  (:Pressed
    (Default|GrabActor _leftcontroller))
  (:Released
    (Default|ReleaseActor _leftcontroller)))

(event Input|ActionEvents|InputActionGrabRight
  (params (Key :type Key%20Structure))
  (bind _rightcontroller (Variables|Default|GetRightController))
  ;[1 1 1] 우측 컨트롤러 입력
  (:Pressed
    (Default|GrabActor _rightcontroller))
  (:Released
    (Default|ReleaseActor _rightcontroller)))

(event Input|ActionEvents|InputAction늘리기(좌)
  (params (Key :type Key%20Structure))
  ;[1 1 1] 좌측 컨트롤러 입력
  (:Pressed
    (Default|FireHand (Variables|Default|GetLeftController))))

(event Input|ActionEvents|InputAction늘리기(우)
  (params (Key :type Key%20Structure))
  ;[1 1 1] 우측 컨트롤러 입력
  (:Pressed
    (Default|FireHand (Variables|Default|GetRightController))))

(fn ConstructionScript)