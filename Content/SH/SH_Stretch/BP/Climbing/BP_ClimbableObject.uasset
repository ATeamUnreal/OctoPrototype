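; BP_ClimbableObject is a VR climbable actor that moves the player's BP_Pawn1 as gripping hands pull on it.
; Climbing and Letgo track up to two motion controllers, update the pawn's ClimbingHands count and re-anchor PivotPoint to the active hand, favoring the second grip.
; While the pawn is climbing, Tick offsets it by the hand's drift from PivotPoint, then pins that controller back to the pivot.
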(event EventBeginPlay)

(event Collision|EventActorBeginOverlap
  (params (OtherActor :type Actor%20Object%20Reference)))

(event EventTick
  (params (DeltaSeconds :type Float%20%28single-precision%29))
  (bind _firstmotioncontroller (Variables|Default|GetFirstMotionController))
  (bind _firstmotioncontroller_2 (Variables|Default|GetFirstMotionController))
  (bind _secondmotioncontroller (Variables|Default|GetSecondMotionController))
  (bind _secondmotioncontroller_2 (Variables|Default|GetSecondMotionController))
  (bind _returnvalue (Utilities|IsValid _secondmotioncontroller_2))
  (bind _returnvalue_2 (select _returnvalue _secondmotioncontroller _firstmotioncontroller_2))
  (Utilities|IsValid (Variables|Default|GetVRPawn)
    (:Is%20Valid
      (if true
        (Utilities|IsValid _firstmotioncontroller
          (:Is%20Valid
            (if (and (Variables|/Game/SH/SH_Stretch/BP/BP_Pawn1.BP_Pawn1_C|GetIsClimbing (Variables|Default|GetVRPawn)) (Rendering|IsVisible _firstmotioncontroller))
              (Transformation|AddActorWorldOffset (Variables|Default|GetVRPawn) (- (Variables|Default|GetPivotPoint) (Transformation|GetWorldLocation _returnvalue_2)))
              (Transformation|SetWorldLocation _returnvalue_2 (Variables|Default|GetPivotPoint) false false))))))))

(event EventClimbing
  (params (Motion%20Controller :type Scene%20Component%20Object%20Reference))
  (if (Utilities|IsValid (Variables|Default|GetFirstMotionController))
    (Variables|Default|SetSecondMotionController Motion%20Controller)
    (else
      (Variables|Default|SetFirstMotionController Motion%20Controller)))
  (Variables|Default|SetPivotPoint (Transformation|GetWorldLocation (select (Utilities|IsValid (Variables|Default|GetSecondMotionController)) (Variables|Default|GetSecondMotionController) (Variables|Default|GetFirstMotionController))))
  (bind _asbp_pawn_1 (Utilities|Casting|CastToBP_Pawn1 (Game|Player|GetPlayerPawn 0)))
  (bind _output_get (Variables|Default|SetVRPawn _asbp_pawn_1))
  (Math|Integer|IncrementInt (Variables|/Game/SH/SH_Stretch/BP/BP_Pawn1.BP_Pawn1_C|GetClimbingHands _output_get)))

(event EventLetgo
  (params (Motion%20Controller :type Scene%20Component%20Object%20Reference))
  (if (Utilities|IsValid (Variables|Default|GetSecondMotionController))
    (if (== Motion%20Controller (Variables|Default|GetSecondMotionController))
      (Variables|Default|SetSecondMotionController 0)
      (Variables|Default|SetPivotPoint (Transformation|GetWorldLocation (Variables|Default|GetFirstMotionController)))
      (else
        (Variables|Default|SetFirstMotionController (Variables|Default|GetSecondMotionController))
        (Variables|Default|SetSecondMotionController 0)
        (Variables|Default|SetPivotPoint (Transformation|GetWorldLocation (Variables|Default|GetFirstMotionController)))))
    (Math|Integer|DecrementInt (Variables|/Game/SH/SH_Stretch/BP/BP_Pawn1.BP_Pawn1_C|GetClimbingHands (Variables|Default|GetVRPawn)) :!label _label)
    (elif (== Motion%20Controller (Variables|Default|GetFirstMotionController))
      (Variables|Default|SetFirstMotionController 0)
      (Variables|Default|SetSecondMotionController 0)
      (Variables|Default|SetPivotPoint "0, 0, 0")
      (goto _label))))

(fn ConstructionScript)