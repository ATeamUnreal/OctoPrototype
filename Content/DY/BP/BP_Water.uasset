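; BP_Water is a water actor that rises steadily from the moment play begins.
; BeginPlay sets the Rising flag, derives a constant speed from the FullZ to InitialZ height difference over Time, and prints it for debugging.
; While Rising is set, Tick moves the actor along local Z by that speed scaled by delta time, with no check to stop at FullZ.
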(event EventBeginPlay
  (Variables|Default|SetRising true)
  (bind _output_get (Variables|Default|Setspeed (/ (- (Variables|Default|GetFullZ) (Variables|Default|GetInitialZ)) (Variables|Default|GetTime))))
  (Development|PrintString (Utilities|String|ToString(Float) _output_get)))

(event EventTick
  (params (DeltaSeconds :type Float%20%28single-precision%29))
  (if (Variables|Default|GetRising)
    (Transformation|AddActorLocalOffset (Math|Vector|MakeVector 0.0 0.0 (* DeltaSeconds (Variables|Default|Getspeed))) false false)))

(fn ConstructionScript)