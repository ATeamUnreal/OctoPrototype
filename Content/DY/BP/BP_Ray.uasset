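; BP_Ray is a laser pointer actor that shows a beam when it points at UI.
; Each Tick it line-traces 200 units along its forward vector against one object type and hides the Ray component when nothing is hit.
; On a hit it reveals Ray, or if already visible, stretches it along X to the hit distance and offsets it by half that distance.
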(event EventTick
  (params (DeltaSeconds :type Float%20%28single-precision%29))
  (bind _ray (Variables|Default|GetRay))
  (bind _ray_2 (Variables|Default|GetRay))
  ;[1 1 1] UI체크를 위한 LineTrace
  (bind (_outhit _returnvalue) (Collision|LineTraceForObjects "0, 0, 0" (+ (Transformation|GetActorLocation) (* (Transformation|GetActorForwardVector) 2e+02)) (Utilities|Array|MakeArray "ObjectTypeQuery7") false 0 "None"))
  (if _returnvalue
    (if (Rendering|IsVisible _ray)
      ;[1 1 1] UI 레이저 모델 업데이트
      (Transformation|SetRelativeScale3D _ray_2 (Math|Vector|MakeVector (Math|Vector|Distance(Vector) (.Location (Collision|BreakHitResult _outhit)) (Transformation|GetActorLocation)) 1.0 1.0))
      (Transformation|SetRelativeLocation _ray_2 (Math|Vector|MakeVector (/ (Math|Vector|Distance(Vector) (.Location (Collision|BreakHitResult _outhit)) (Transformation|GetActorLocation)) 2.0) 0.0 0.0) false false)
      (else
        (Rendering|SetVisibility _ray true false)))
    (else
      (Rendering|SetVisibility _ray false false))))

(fn ConstructionScript)