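; BP_Button is a physical push button that gets pushed down by whatever component overlaps it.
; It stores the first overlapping component and its contact height, clearing it when that overlap ends.
; Tick lowers the button by that component's downward world-Z travel until it reaches the pressed threshold and sets Pressed.
; Nothing in the graph resets Pressed or returns the button to its starting height.
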(event OnComponentBeginOverlap(Button)
  (params (OverlappedComponent :type Primitive%20Component%20Object%20Reference) (OtherActor :type Actor%20Object%20Reference) (OtherComp :type Primitive%20Component%20Object%20Reference) (OtherBodyIndex :type Integer) (bFromSweep :type Boolean) (SweepResult :type Hit%20Result%20Structure%20%28by%20ref%29))
  ;[1 1 1] Press
  (Utilities|IsValid (Variables|Default|GetOverlapedComponent)
    (:Is%20Not%20Valid
      (bind _output_get (Variables|Default|SetOverlapedComponent OtherComp))
      (Variables|Default|SetContactedLocationZ (.z (Transformation|GetWorldLocation _output_get))))))

(event OnComponentEndOverlap(Button)
  (params (OverlappedComponent :type Primitive%20Component%20Object%20Reference) (OtherActor :type Actor%20Object%20Reference) (OtherComp :type Primitive%20Component%20Object%20Reference) (OtherBodyIndex :type Integer))
  ;[1 1 1] Release
  (if (== OtherComp (Variables|Default|GetOverlapedComponent))
    (Variables|Default|SetOverlapedComponent 0)))

(event EventBeginPlay
  ;[1 1 1] 초기화
  (Variables|Default|SetInitialLocationZ (.z (Variables|/Script/Engine.SceneComponent|GetRelativeLocation (Variables|Default|GetButton)))))

(event EventTick
  (params (DeltaSeconds :type Float%20%28single-precision%29))
  (if (not (Variables|Default|GetPressed))
    (Utilities|IsValid (Variables|Default|GetOverlapedComponent)
      (:Is%20Valid
        (Variables|Default|SetCurrentLocationZ (- (Variables|Default|GetInitialLocationZ) (- (Variables|Default|GetContactedLocationZ) (.z (Transformation|GetWorldLocation (Variables|Default|GetOverlapedComponent))))))
        (if (<= (Variables|Default|GetCurrentLocationZ) (Variables|Default|GetPressedLocationZ))
          (Variables|Default|SetPressed true)
          (elif (< (Variables|Default|GetCurrentLocationZ) (Variables|Default|GetInitialLocationZ))
            (Transformation|SetRelativeLocation (Variables|Default|GetButton) (Math|Vector|MakeVector 0.0 0.0 (Variables|Default|GetCurrentLocationZ)) false false)))))))

(fn ConstructionScript)