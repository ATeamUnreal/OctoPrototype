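; BP_Letter is an actor that shows a text string as a row of 3D letter meshes that break loose on overlap.
; On BeginPlay it spawns an attached BP_Char per uppercased character, using A–Z mesh lookup and a palette color, centers the row and sizes the Box.
; Box overlap enables physics on the letters, then calls an empty OnButtonClick event after a short delay.
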(event OnComponentBeginOverlap(Box)
  (params (OverlappedComponent :type Primitive%20Component%20Object%20Reference) (OtherActor :type Actor%20Object%20Reference) (OtherComp :type Primitive%20Component%20Object%20Reference) (OtherBodyIndex :type Integer) (bFromSweep :type Boolean) (SweepResult :type Hit%20Result%20Structure%20%28by%20ref%29))
  (Development|PrintString (Utilities|GetDisplayName OtherActor))
  (for _array_element (Actor|GetAttachedActors)
    (bind _asbp_char (Utilities|Casting|CastToBP_Char _array_element))
    (Collision|SetCollisionEnabled (Variables|/Game/DY/UITest/BP/BP_Char.BP_Char_C|GetStaticMesh _asbp_char) "QueryAndPhysics")
    (Physics|SetSimulatePhysics (Variables|/Game/DY/UITest/BP/BP_Char.BP_Char_C|GetStaticMesh _asbp_char) true)
    (Utilities|FlowControl|Delay 1.0)
    (CallFunction|OnButtonClick)))

(event Custom|SetText
  ;[1 1 1] 알파벳 글자 생성 + 배치
  (Variables|Default|SetSize (Utilities|Array|Length (Utilities|String|GetCharacterArrayfromString (Variables|Default|GetText))))
  (for (_array_element _array_index) (Utilities|String|GetCharacterArrayfromString (Class|KismetStringLibrary|ToUpper (Variables|Default|GetText)))
    (bind _outputpin (CallFunction|FindLetterMesh _array_element))
    (Transformation|SetActorRelativeLocation _outputpin (Math|Vector|MakeVector 0.0 (+ (* (* (Variables|Default|GetSize) (Variables|Default|GetSpace)) 0.5) (* _array_index (* (Variables|Default|GetSpace) -1.0)) (* (Variables|Default|GetSpace) 0.5 -1.0)) 0.0)))
  (Components|Box|SetBoxExtent (Variables|Default|GetBox) (Math|Vector|MakeVector 2e+01 (* (Variables|Default|GetSize) 32.5) 5e+01) false))

(event Custom|OnButtonClick)

(event EventBeginPlay
  (CallFunction|SetText))

(fn ConstructionScript)

(fn FindLetterMesh
  (params (SourceString :type String))
  (Variables|Default|SetcurLetter (- (Utilities|String|GetCharacterasNumber SourceString) 65))
  (if (< (Variables|Default|GetcurLetter) 26)
    (bind _returnvalue (Game|SpawnActorfromClass "/Game/DY/UITest/BP/BP_Char.BP_Char_C" (Transformation|GetActorTransform) "AlwaysSpawn" 0 0))
    (Transformation|AttachActorToActor _returnvalue self "None" "SnapToTarget" "SnapToTarget" "KeepRelative" false)
    (Components|StaticMesh|SetStaticMesh (Variables|/Game/DY/UITest/BP/BP_Char.BP_Char_C|GetStaticMesh _returnvalue) (Utilities|Array|Get(acopy) (Variables|Default|GetLetters) (Variables|Default|GetcurLetter)))
    (Rendering|Material|SetScalarParameterValueonMaterials (Variables|/Game/DY/UITest/BP/BP_Char.BP_Char_C|GetStaticMesh _returnvalue) "Color" (Variables|Default|GetPalletteColor))
    (return _returnvalue)
    (else
      (return 0))))