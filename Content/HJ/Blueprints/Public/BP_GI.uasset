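; BP_GI, apparently the game instance, responds to network failures with on-screen feedback.
; HandleNetworkError prints the failure type and server flag, then uses a DoOnce to create and show a NetworkErrorWidget for the first player controller.
; GotoStart is an empty event; the branch opening VRStart for servers or TPSStart for clients is disconnected and never runs, as is a switch on failure type.
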(event Custom|GotoStart
  (params (IsServer :type Boolean)))

(event EventHandleNetworkError
  (params (FailureType :type ENetworkFailure%20Enum :default "NetDriverAlreadyExists") (bIsServer :type Boolean))
  (Development|PrintString (Utilities|String|EnumtoString FailureType) true true "(R=0.000000,G=0.660000,B=1.000000,A=1.000000)" 1e+01)
  (Development|PrintString (Utilities|String|ToString(Boolean) bIsServer) true true "(R=1.000000,G=0.087969,B=0.000000,A=1.000000)" 1e+01)
  (Utilities|FlowControl|DoOnce false
    (:Completed
      (bind _returnvalue (UserInterface|CreateWidget "/Game/HJ/Blueprints/Public/NetworkErrorWidget.NetworkErrorWidget_C" (Game|GetPlayerController 0)))
      (UserInterface|Viewport|AddtoViewport _returnvalue 0))))